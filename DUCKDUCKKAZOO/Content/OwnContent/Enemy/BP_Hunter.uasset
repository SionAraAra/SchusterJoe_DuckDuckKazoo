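; BP_Hunter is an enemy that shoots at a BP_Duck inside its box overlap range.
; Each tick with the duck in range and gun loaded, a random roll either sets the duck's Die flag or starts a two-second reload.
; When IsHit is set, it nudges along Hit, spawns a replacement near randomly picked BP_HunterSpawn actors, drops a BP_Berry and destroys itself.
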(event `self.ReceiveBeginPlay`
  (`|ExecutionSequence`
    (:`then_0`
      (bind _outactors (`GameplayStatics.GetAllActorsOfClass` "/Game/OwnContent/Enemy/BP_HunterSpawn.BP_HunterSpawn_C"))
      (set `self.HunterSpawnArray` _outactors)
      (set `self.Hunter` self))))

(event `self.ReceiveTick`
  (params (DeltaSeconds :type "Float (single-precision)"))
  (bind (_returnvalue_x _returnvalue_y) (`KismetMathLibrary.BreakVector` (`self.K2_GetActorLocation`)))
  (bind (_hit_x _hit_y) (`KismetMathLibrary.BreakVector` (`self.Hit`)))
  (bind (_returnvalue_x_2 _returnvalue_y_2) (`KismetMathLibrary.BreakVector2D` (`KismetMathLibrary.Vector2DInterpTo` (`KismetMathLibrary.MakeVector2D` _returnvalue_x _returnvalue_y) (`KismetMathLibrary.MakeVector2D` (+ _returnvalue_x _hit_x) (+ _returnvalue_y _hit_y)) (`self.Delta Time`) 0.2)))
  (bind _returnvalue (`self.GetTransform` (`|GetArrayItem` (`self.HunterSpawnArray`) (`KismetMathLibrary.RandomIntegerInRange` 0 4))))
  (set `self.Delta Time` DeltaSeconds)
  (`|ExecutionSequence`
    (:`then_0`
      ; respawn
      (if (`self.IsHit`)
        (set `self.IsHit` false)
        (`self.K2_SetActorLocation` (`KismetMathLibrary.MakeVector` _returnvalue_x_2 _returnvalue_y_2))
        (`|ExecutionSequence`
          (:`then_0`
            (`KismetSystemLibrary.PrintString` "Delay Over")
            (`|SpawnActorFromClass` "BP_Hunter_C" (`KismetMathLibrary.MakeTransform` (`KismetMathLibrary.MakeVector` (+ (.x (.location _returnvalue)) 100.0) (+ (.y (.location _returnvalue)) -250.0) (.z (.location _returnvalue))) (.rotation _returnvalue) (.scale _returnvalue)) "AdjustIfPossibleButAlwaysSpawn" "MultiplyWithRoot" (`self.Hunter`) null))
          (:`then_1`
            (`|SpawnActorFromClass` "/Game/OwnContent/Berry/BP_Berry.BP_Berry_C" (`self.GetTransform`) "AlwaysSpawn" "MultiplyWithRoot" null null)
            (`KismetSystemLibrary.PrintString` "Spawned berry"))
          (:`then_2`
            (`self.K2_DestroyActor`)))))
    (:`then_1`
      ; Shooting Duck
      (if (`self.InRange`)
        (if (`self.GunLoaded`)
          (if (== (`KismetMathLibrary.RandomIntegerInRange` 0 3) 0)
            (set `/Game/OwnContent/Player/BP_Duck.Die` true (`self.Duck`))
            (`KismetSystemLibrary.PrintString` "YOU HIT")
            (else
              (set `self.GunLoaded` false)
              (`KismetSystemLibrary.Delay` 2.0)
              (set `self.GunLoaded` true)
              (`KismetSystemLibrary.PrintString` "YOU MISSED"))))))))

(event `self.Box.OnComponentBeginOverlap`
  (params (OverlappedComponent :type "PrimitiveComponent Object Reference") (OtherActor :type "Actor Object Reference") (OtherComp :type "PrimitiveComponent Object Reference") (OtherBodyIndex :type Integer) (bFromSweep :type Boolean) (SweepResult :type "HitResult Structure (by ref)"))
  (bind _asbp_duck (cast `/Game/OwnContent/Player/BP_Duck` OtherActor))
  (set `self.Duck` _asbp_duck)
  (set `self.InRange` true))

(event `self.Box.OnComponentEndOverlap`
  (params (OverlappedComponent :type "PrimitiveComponent Object Reference") (OtherActor :type "Actor Object Reference") (OtherComp :type "PrimitiveComponent Object Reference") (OtherBodyIndex :type Integer))
  (if (== OtherActor (`self.Duck`))
    (set `self.InRange` false)))

(fn `UserConstructionScript`)